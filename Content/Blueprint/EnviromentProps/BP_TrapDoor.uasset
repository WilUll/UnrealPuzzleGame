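; BP_TrapDoor is an environment prop trap door that swings between a flat and a 90-degree pitch position when activated or deactivated.
; Activate and Deactivate wait a configurable delay, play a piston sound, then set the swing direction from StartDown, with Deactivate reversing Activate.
; Tick eases the pivot Scene component's pitch toward the target with FInterpTo, snapping and stopping once within a small tolerance.
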(event EventBeginPlay)

(event EventActivate
  (Utilities|FlowControl|Delay (Variables|Default|GetStartDelay))
  (Audio|PlaySoundatLocation "/Game/Audio/Piston.Piston" (Transformation|GetWorldLocation (Variables|Default|GetCube)) "0, 0, 0" 1.0 1.0 0.0 0 0 0 0)
  (if (Variables|Default|GetStartDown)
    (Variables|Default|SetGoUp true)
    (else
      (Variables|Default|SetGoUp false)))
  (Variables|Default|SetStartMoving true))

(event EventDeactivate
  (Utilities|FlowControl|Delay (Variables|Default|GetExitDelay))
  (Audio|PlaySoundatLocation "/Game/Audio/Piston.Piston" (Transformation|GetWorldLocation (Variables|Default|GetCube)) "0, 0, 0" 1.0 1.0 0.0 0 0 0 0)
  (if (Variables|Default|GetStartDown)
    (Variables|Default|SetGoUp false)
    (else
      (Variables|Default|SetGoUp true)))
  (Variables|Default|SetStartMoving true))

(event EventTick
  (params (DeltaSeconds :type Float%20%28single-precision%29))
  (bind _scene (Variables|Default|GetScene))
  (bind _scene_2 (Variables|Default|GetScene))
  (bind _scene_3 (Variables|Default|GetScene))
  (bind _relativerotation (Variables|/Script/Engine.SceneComponent|GetRelativeRotation _scene_2))
  (if (Variables|Default|GetStartMoving)
    (if (Variables|Default|GetGoUp)
      (Transformation|SetRelativeRotation _scene (Math|Rotator|MakeRotator 0.0 (Math|Interpolation|FInterpTo (.pitch _relativerotation) 0.0 DeltaSeconds 2.0) 0.0) false false)
      (if (Math|Float|NearlyEqual(Float) (.pitch (Variables|/Script/Engine.SceneComponent|GetRelativeRotation _scene)) 0.0 0.5)
        (Transformation|SetRelativeRotation _scene_3 (Math|Rotator|MakeRotator 0.0 0.0 0.0) false false)
        (Variables|Default|SetStartMoving false :!label _label))
      (else
        (Transformation|SetRelativeRotation _scene (Math|Rotator|MakeRotator 0.0 (Math|Interpolation|FInterpTo (.pitch _relativerotation) 9e+01 DeltaSeconds 2.0) 0.0) false false)
        (if (Math|Float|NearlyEqual(Float) (.pitch (Variables|/Script/Engine.SceneComponent|GetRelativeRotation _scene)) 9e+01 0.5)
          (Transformation|SetRelativeRotation _scene_3 (Math|Rotator|MakeRotator 0.0 9e+01 0.0) false false)
          (goto _label))))))

(fn ConstructionScript)