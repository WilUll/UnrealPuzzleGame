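; BP_Piston is an environment prop whose cylinder rises while a required number of linked buttons are pressed.
; Delayed Activate and Deactivate events keep a count of pressed buttons and set the raise flag only when it exactly matches the needed count.
; Tick uses VInterpTo to ease the cylinder between its BeginPlay location and that location plus an offset, without sweeping.
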(event EventBeginPlay
  (Variables|Default|SetStartLocation (Transformation|GetWorldLocation (Variables|Default|GetCylinder))))

(event EventDeactivate
  (Utilities|FlowControl|Delay (Variables|Default|GetExitDelay))
  (bind _output_get (Variables|Default|SetCurretButtonsPressed (- (Variables|Default|GetCurretButtonsPressed) 1)))
  (if (!= _output_get (Variables|Default|GetNeededButtonsPressed))
    (Variables|Default|SetTimeToGoUp false)))

(event EventActivate
  (Utilities|FlowControl|Delay (Variables|Default|GetStartDelay))
  (bind _output_get (Variables|Default|SetCurretButtonsPressed (+ (Variables|Default|GetCurretButtonsPressed) 1)))
  (if (== _output_get (Variables|Default|GetNeededButtonsPressed))
    (Variables|Default|SetTimeToGoUp true)))

(event EventTick
  (params (DeltaSeconds :type Float%20%28single-precision%29))
  (bind _cylinder (Variables|Default|GetCylinder))
  (if (Variables|Default|GetTimeToGoUp)
    (Transformation|SetWorldLocation _cylinder (Math|Interpolation|VInterpTo (Transformation|GetWorldLocation _cylinder) (+ (Variables|Default|GetStartLocation) (Variables|Default|GetLerpValue)) DeltaSeconds 1.0) false false)
    (else
      (Transformation|SetWorldLocation _cylinder (Math|Interpolation|VInterpTo (Transformation|GetWorldLocation (Variables|Default|GetCylinder)) (Variables|Default|GetStartLocation) DeltaSeconds 1.0) false false))))

(fn ConstructionScript)