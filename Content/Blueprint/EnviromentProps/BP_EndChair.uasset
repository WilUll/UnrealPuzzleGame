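; BP_EndChair is an interactable chair prop that, judging by its name, seats the player at an ending.
; Interact calls Activate, which disables player movement, turns the look rotation 180 degrees and moves the player to the chair's root, raised by the player's half height.
; After a short delay, it sends ActivateMessage to every entry in ActivatableObjects to trigger linked objects.
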(event EventActivate
  (bind _player (Variables|Default|GetPlayer))
  (Pawn|Components|CharacterMovement|DisableMovement (Variables|/Script/Engine.Character|GetCharacterMovement _player))
  (Variables|/Game/Blueprint/PlayerStuff/Player/BP_Player.BP_Player_C|SetLookRotationX _player (+ (Variables|/Game/Blueprint/PlayerStuff/Player/BP_Player.BP_Player_C|GetLookRotationX _player) 1.8e+02))
  (Transformation|SetActorLocation _player (+ (Transformation|GetWorldLocation (Variables|Default|GetDefaultSceneRoot)) (Math|Vector|MakeVector 0.0 0.0 (Variables|/Game/Blueprint/PlayerStuff/Player/BP_Player.BP_Player_C|GetPlayerHeightHalf _player))) false false)
  (Utilities|FlowControl|Delay 0.5)
  (for _array_element (Variables|Default|GetActivatableObjects)
    (Class|IBPActivateable|Activate(Message) _array_element)))

(fn ConstructionScript)

(fn Interact
  (CallFunction|Activate))