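; BP_TriggerTimer is an environment prop that switches the ActorToActivate list on and off through activate and deactivate messages.
; Without UsingTrigger, a Tick countdown repeatedly activates them, then deactivates them after a delay.
; With it, Box overlaps by \"Box\" or \"Player\" tags activate, but only \"Box\" exits deactivate.
; Delays sit inside the ForEach loops, so trigger mode effectively messages only the last actor.
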(event OnComponentBeginOverlap(Box)
  (params (OverlappedComponent :type Primitive%20Component%20Object%20Reference) (OtherActor :type Actor%20Object%20Reference) (OtherComp :type Primitive%20Component%20Object%20Reference) (OtherBodyIndex :type Integer) (bFromSweep :type Boolean) (SweepResult :type Hit%20Result%20Structure%20%28by%20ref%29))
  (if (Variables|Default|GetUsingTrigger)
    (if (Math|Boolean|ORBoolean (Actor|ActorHasTag OtherActor "Box") (Components|ComponentHasTag OtherComp "Box") (Actor|ActorHasTag OtherActor "Player"))
      (for _array_element (Variables|Default|GetActorToActivate)
        (Utilities|FlowControl|Delay (Variables|Default|GetStartDelayForTrigger))
        (Class|IBPActivateable|Activate(Message) _array_element)))))

(event OnComponentEndOverlap(Box)
  (params (OverlappedComponent :type Primitive%20Component%20Object%20Reference) (OtherActor :type Actor%20Object%20Reference) (OtherComp :type Primitive%20Component%20Object%20Reference) (OtherBodyIndex :type Integer))
  (if (Variables|Default|GetUsingTrigger)
    (if (or (Actor|ActorHasTag OtherActor "Box") (Components|ComponentHasTag OtherComp "Box"))
      (for _array_element (Variables|Default|GetActorToActivate)
        (Utilities|FlowControl|Delay (Variables|Default|GetDelayTimeForTrigger))
        (Class|IBPActivateable|Deactivate(Message) _array_element)))))

(event EventTick
  (params (DeltaSeconds :type Float%20%28single-precision%29))
  (if (not (Variables|Default|GetUsingTrigger))
    (Variables|Default|SetTimer (- (Variables|Default|GetTimer) DeltaSeconds))
    (if (<= (Variables|Default|GetTimer) 0.0)
      (Variables|Default|SetTimer (Variables|Default|GetStartTime))
      (for _array_element (Variables|Default|GetActorToActivate)
        (Class|IBPActivateable|Activate(Message) _array_element)
        (Utilities|FlowControl|Delay (Variables|Default|GetDelayTime))
        (for _array_element_2 (Variables|Default|GetActorToActivate)
          (Class|IBPActivateable|Deactivate(Message) _array_element_2))))))

(event EventBeginPlay
  (Variables|Default|SetStartTime (Variables|Default|GetTimer)))

(fn ConstructionScript)