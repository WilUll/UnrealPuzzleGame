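; BP_NormalBox is an interactable physics box prop that can return to its starting location.
; Interact toggles IsInteracting and returns it, switching the cube's physics simulation and collision off while interacting and back on afterwards.
; BeginPlay stores the start location, and Respawn moves the cube there, clears the flag and restarts physics without restoring collision.
; The cube wakes its rigid bodies whenever it falls asleep, so it stays awake.
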(event OnComponentSleep(Cube)
  (params (SleepingComponent :type Primitive%20Component%20Object%20Reference) (BoneName :type Name :default "None"))
  (Class|PrimitiveComponent|WakeAllRigidBodies SleepingComponent))

(event EventBeginPlay
  (Variables|Default|SetStartLocation (Transformation|GetWorldLocation (Variables|Default|GetCube))))

(event Collision|EventActorBeginOverlap
  (params (OtherActor :type Actor%20Object%20Reference)))

(event EventTick
  (params (DeltaSeconds :type Float%20%28single-precision%29)))

(event EventRespawn
  (Variables|Default|SetIsInteracting false)
  (Transformation|SetWorldLocation (Variables|Default|GetCube) (Variables|Default|GetStartLocation) false false)
  (Physics|SetSimulatePhysics (Variables|Default|GetCube) false)
  (Physics|SetSimulatePhysics (Variables|Default|GetCube) true))

(fn ConstructionScript)

(fn Interact
  (bind _cube (Variables|Default|GetCube))
  (if (Variables|Default|GetIsInteracting)
    (Physics|SetSimulatePhysics _cube true)
    (Collision|SetCollisionEnabled _cube "QueryAndPhysics")
    (bind _output_get (Variables|Default|SetIsInteracting false))
    (return _output_get)
    (else
      (Physics|SetSimulatePhysics _cube false)
      (Collision|SetCollisionEnabled _cube "NoCollision")
      (bind _output_get_2 (Variables|Default|SetIsInteracting true))
      (return _output_get_2))))