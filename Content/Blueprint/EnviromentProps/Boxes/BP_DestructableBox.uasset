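; Destructible box prop that loses health on impact after being interacted with and respawns at its start location.
; Interact toggles an interacting state, during which Tick re-enables physics on a sleeping cube and re-arms a DoOnce gate.
; Component hits pass that gate once, costing health if the box is no longer being interacted with.
; At zero health the box returns to its BeginPlay location, restarts physics and refills health.
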(event OnComponentHit(Cube)
  (params (HitComponent :type Primitive%20Component%20Object%20Reference) (OtherActor :type Actor%20Object%20Reference) (OtherComp :type Primitive%20Component%20Object%20Reference) (NormalImpulse :type Vector :default "0, 0, 0") (Hit :type Hit%20Result%20Structure%20%28by%20ref%29))
  (Utilities|FlowControl|DoOnce false
    (:Completed
      (if (not (Variables|Default|GetIsInteracting))
        (Variables|Default|SetHealth (- (Variables|Default|GetHealth) 1))
        (if (== (Variables|Default|GetHealth) 0)
          (CallFunction|Respawn)
          (Variables|Default|SetHealth 3))))))

(event EventBeginPlay
  (Variables|Default|SetStartLocation (Transformation|GetWorldLocation (Variables|Default|GetCube))))

(event EventRespawn
  (Transformation|SetWorldLocation (Variables|Default|GetCube) (Variables|Default|GetStartLocation) false false)
  (Physics|SetSimulatePhysics (Variables|Default|GetCube) false)
  (Physics|SetSimulatePhysics (Variables|Default|GetCube) true)
  (Variables|Default|SetIsInteracting false))

(event EventTick
  (params (DeltaSeconds :type Float%20%28single-precision%29))
  (if (Variables|Default|GetIsInteracting)
    (Utilities|FlowControl|Sequence
      (:then_0
        (if (not (Class|PrimitiveComponent|IsAnyRigidBodyAwake (Variables|Default|GetCube)))
          (Physics|SetSimulatePhysics (Variables|Default|GetCube) true)))
      (:then_1
        (Utilities|FlowControl|DoOnce false) ; enters at Reset
      ))))

(fn ConstructionScript)

(fn Interact
  (if (Variables|Default|GetIsInteracting)
    (bind _output_get (Variables|Default|SetIsInteracting false))
    (return _output_get)
    (else
      (bind _output_get_2 (Variables|Default|SetIsInteracting true))
      (return _output_get_2))))