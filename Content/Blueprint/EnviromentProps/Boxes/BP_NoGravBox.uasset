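; BP_NoGravBox is an environment box prop that can be picked up and dropped, with physics simulated only while held.
; Interact toggles IsInteracting and the Cube's physics simulation, prints the action and returns the new state.
; While interacting, Tick re-applies physics simulation whenever no rigid body on the Cube is awake.
; Respawn moves the Cube to its BeginPlay location, toggles physics on then off, and clears IsInteracting.
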(event EventBeginPlay
  (Variables|Default|SetStartLocation (Transformation|GetWorldLocation (Variables|Default|GetCube))))

(event Collision|EventActorBeginOverlap
  (params (OtherActor :type Actor%20Object%20Reference)))

(event EventTick
  (params (DeltaSeconds :type Float%20%28single-precision%29))
  (if (Variables|Default|GetIsInteracting)
    (if (not (Class|PrimitiveComponent|IsAnyRigidBodyAwake (Variables|Default|GetCube)))
      (Physics|SetSimulatePhysics (Variables|Default|GetCube) true))))

(event EventRespawn
  (Transformation|SetWorldLocation (Variables|Default|GetCube) (Variables|Default|GetStartLocation) false false)
  (Physics|SetSimulatePhysics (Variables|Default|GetCube) true)
  (Physics|SetSimulatePhysics (Variables|Default|GetCube) false)
  (Variables|Default|SetIsInteracting false))

(fn ConstructionScript)

(fn Interact
  (if (Variables|Default|GetIsInteracting)
    (Development|PrintString "Dropping")
    (bind _output_get (Variables|Default|SetIsInteracting false))
    (Physics|SetSimulatePhysics (Variables|Default|GetCube) false)
    (return _output_get)
    (else
      (Development|PrintString "Picking Up")
      (bind _output_get_2 (Variables|Default|SetIsInteracting true))
      (Physics|SetSimulatePhysics (Variables|Default|GetCube) true)
      (return _output_get_2))))