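; Interactable environment button that, when used, temporarily activates the objects in its ActivatableObject list.
; Interact sets a flag that lets Tick ease the Cube along local Y to its pressed position with FInterpTo, then back out before re-arming.
; On reaching the pressed position, ButtonDown sends ActivateMessage to each linked object, with DeactivateMessage following after a fixed delay placed inside the loop.
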(event Custom|ButtonDown
  (for _array_element (Variables|Default|GetActivatableObject)
    (Class|IBPActivateable|Activate(Message) _array_element)
    (Utilities|FlowControl|Delay 5.0)
    (for _array_element_2 (Variables|Default|GetActivatableObject)
      (Class|IBPActivateable|Deactivate(Message) _array_element_2))))

(event EventBeginPlay)

(event Collision|EventActorBeginOverlap
  (params (OtherActor :type Actor%20Object%20Reference)))

(event EventTick
  (params (DeltaSeconds :type Float%20%28single-precision%29))
  (bind _cube (Variables|Default|GetCube))
  (bind _cube_2 (Variables|Default|GetCube))
  (bind _relativelocation (Variables|/Script/Engine.SceneComponent|GetRelativeLocation _cube))
  (bind _returnvalue (Math|Interpolation|FInterpTo (.y _relativelocation) 0.0 DeltaSeconds 2.5))
  (bind _returnvalue_2 (Math|Interpolation|FInterpTo (.y _relativelocation) 5.0 DeltaSeconds 2.5))
  (if (Variables|Default|GetInteracted)
    (if (Variables|Default|GetIsDown)
      (Transformation|SetRelativeLocation _cube_2 (Math|Vector|MakeVector 0.0 _returnvalue_2 0.0) false false)
      (if (Math|Float|NearlyEqual(Float) _returnvalue_2 5.0 0.1)
        (Variables|Default|SetInteracted false)
        (Variables|Default|SetIsDown false))
      (else
        (Transformation|SetRelativeLocation _cube_2 (Math|Vector|MakeVector 0.0 _returnvalue 0.0) false false)
        (if (Math|Float|NearlyEqual(Float) _returnvalue 0.0 0.1)
          (Variables|Default|SetIsDown true)
          (CallFunction|ButtonDown))))))

(fn ConstructionScript)

(fn Interact
  (if (not (Variables|Default|GetInteracted))
    (Variables|Default|SetInteracted true)
    (return false)))