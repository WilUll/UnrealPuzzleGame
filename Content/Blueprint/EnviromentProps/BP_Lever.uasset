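; BP_Lever is an interactable lever prop that switches a referenced ActivateableObject on and off.
; Interact sets an Interacted flag, which blocks retriggering while Tick eases the Scene component's roll toward RotateAngle or back to zero with FInterpTo.
; Once the roll is within a loose tolerance of its target, the lever sends the activate or deactivate message, flips IsOn and stops moving.
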(event EventTick
  (params (DeltaSeconds :type Float%20%28single-precision%29))
  (bind _scene (Variables|Default|GetScene))
  (bind _rotateangle (Variables|Default|GetRotateAngle))
  (bind _activateableobject (Variables|Default|GetActivateableObject))
  (bind _relativerotation (Variables|/Script/Engine.SceneComponent|GetRelativeRotation _scene))
  (bind _returnvalue (Math|Interpolation|FInterpTo (.roll _relativerotation) _rotateangle DeltaSeconds 3.0))
  (bind _returnvalue_2 (Math|Interpolation|FInterpTo (.roll _relativerotation) 0.0 DeltaSeconds 3.0))
  (if (Variables|Default|GetInteracted)
    (if (Variables|Default|GetIsOn)
      (Transformation|SetRelativeRotation _scene (Math|Rotator|MakeRotator _returnvalue_2 0.0 0.0) false false)
      (if (Math|Float|NearlyEqual(Float) _returnvalue_2 0.0 1e+01)
        (Class|IBPActivateable|Deactivate(Message) _activateableobject)
        (Variables|Default|SetIsOn false)
        (Variables|Default|SetInteracted false :!label _label))
      (else
        (Transformation|SetRelativeRotation _scene (Math|Rotator|MakeRotator _returnvalue 0.0 0.0) false false)
        (if (Math|Float|NearlyEqual(Float) _returnvalue (Variables|Default|GetRotateAngle) 1e+01)
          (Class|IBPActivateable|Activate(Message) _activateableobject)
          (Variables|Default|SetIsOn true)
          (goto _label))))))

(fn ConstructionScript)

(fn Interact
  (if (not (Variables|Default|GetInteracted))
    (Variables|Default|SetInteracted true)
    (return false)))