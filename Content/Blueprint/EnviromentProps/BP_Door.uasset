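; BP_Door is an environment door that opens once a required number of buttons are pressed.
; Activate and Deactivate adjust a press counter after their own delays.
; Reaching the exact count plays the OpenDoor timeline, and any deactivation while open reverses a separate timeline to close it.
; Both timelines move the Cube by multiplying their vector output with its starting relative location, rather than adding an offset.
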(event EventActivate
  (Utilities|FlowControl|Delay (Variables|Default|GetStartDelay))
  (bind _output_get (Variables|Default|SetCurrentButtonPressed (+ (Variables|Default|GetCurrentButtonPressed) 1)))
  (if (== _output_get (Variables|Default|GetNeededButtonsPressed))
    (bind _vector (Timeline|OpenDoor PlayFromStart)
      (:Update
        (Transformation|SetRelativeLocation (Variables|Default|GetCube) (* _vector (Variables|Default|GetDoorStartVector)) false false)
        (Variables|Default|SetDoorIsOpen true)))))

(event EventDeactivate
  (Utilities|FlowControl|Delay (Variables|Default|GetExitDelay))
  (Variables|Default|SetCurrentButtonPressed (- (Variables|Default|GetCurrentButtonPressed) 1))
  (if (Variables|Default|GetDoorIsOpen)
    (bind _vector (Timeline|Timeline_0 ReverseFromEnd)
      (:Update
        (Transformation|SetRelativeLocation (Variables|Default|GetCube) (* _vector (Variables|Default|GetDoorStartVector)) false false)
        (Variables|Default|SetDoorIsOpen false)))))

(event EventBeginPlay
  (Variables|Default|SetDoorStartVector (Variables|/Script/Engine.SceneComponent|GetRelativeLocation (Variables|Default|GetCube))))

(fn ConstructionScript)