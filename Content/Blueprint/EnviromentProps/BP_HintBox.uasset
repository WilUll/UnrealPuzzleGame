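; BP_HintBox is an environment prop that shows a one-time text hint through a widget component.
; BeginPlay collapses the widget and fills it with HintText.
; After Activate, Tick interpolates it to HintOffset and full scale, waits a configurable Delay, then eases it to the negated offset and collapses it.
; Delay nodes inside Tick drive the state flags; IsDone never resets and Deactivate is empty.
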(event EventBeginPlay
  (bind _widget (Variables|Default|GetWidget))
  (Transformation|SetRelativeScale3D _widget "1.000000, 0, 0")
  (bind _aswbp_hint_text_box (Utilities|Casting|CastToWBP_HintTextBox (UserInterface|GetUserWidgetObject _widget)))
  (Rendering|Components|TextRender|SetText (Variables|/Game/Blueprint/EnviromentProps/WBP_HintTextBox.WBP_HintTextBox_C|GetTextBlock_44 _aswbp_hint_text_box) (Variables|Default|GetHintText)))

(event Collision|EventActorBeginOverlap
  (params (OtherActor :type Actor%20Object%20Reference)))

(event EventTick
  (params (DeltaSeconds :type Float%20%28single-precision%29))
  (bind _returnvalue (Utilities|Time|GetWorldDeltaSeconds))
  (bind _returnvalue_2 (Utilities|Time|GetWorldDeltaSeconds))
  (bind _widget (Variables|Default|GetWidget))
  (bind _widget_2 (Variables|Default|GetWidget))
  (bind _widget_3 (Variables|Default|GetWidget))
  (bind _widget_4 (Variables|Default|GetWidget))
  (if (Variables|Default|GetIsDone)
    (if (not (Variables|Default|GetIsInactive))
      (Transformation|SetRelativeLocation _widget_3 (Math|Interpolation|VInterpTo (Variables|/Script/Engine.SceneComponent|GetRelativeLocation _widget_4) (* (Variables|Default|GetHintOffset) -1.0) _returnvalue_2 1e+01) false false)
      (Transformation|SetRelativeScale3D _widget_3 (Math|Interpolation|VInterpTo (Variables|/Script/Engine.SceneComponent|GetRelativeScale3D _widget_4) "1.000000,0.000000,0.000000" _returnvalue_2 2e+01))
      (Utilities|FlowControl|Delay 1.0)
      (Variables|Default|SetIsInactive true))
    (elif (Variables|Default|GetIsActive)
      (Transformation|SetRelativeLocation _widget_2 (Math|Interpolation|VInterpTo (Variables|/Script/Engine.SceneComponent|GetRelativeLocation _widget) (Variables|Default|GetHintOffset) _returnvalue 1e+01) false false)
      (Transformation|SetRelativeScale3D _widget_2 (Math|Interpolation|VInterpTo (Variables|/Script/Engine.SceneComponent|GetRelativeScale3D _widget) "1.000000,1.000000,1.000000" _returnvalue 1e+01))
      (Utilities|FlowControl|Delay (Variables|Default|GetDelay))
      (Variables|Default|SetIsActive false)
      (Variables|Default|SetIsDone true))))

(event EventActivate
  (Variables|Default|SetIsActive true))

(event EventDeactivate)

(fn ConstructionScript)