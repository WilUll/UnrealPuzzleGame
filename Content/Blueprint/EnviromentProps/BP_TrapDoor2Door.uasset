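; Double-leaf trap door prop that swings open on Activate and closes on Deactivate.
; Both events set a direction flag and enable the Tick logic, which uses FInterpTo to pitch two Scene pivots in opposite directions, or back to level.
; The motion flag clears when the first pivot is within a degree of its target, as the second pivot's check has a negative tolerance.
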(event EventTick
  (params (DeltaSeconds :type Float%20%28single-precision%29))
  (bind _scene (Variables|Default|GetScene))
  (bind _scene1 (Variables|Default|GetScene1))
  (bind _scene_2 (Variables|Default|GetScene))
  (bind _scene1_2 (Variables|Default|GetScene1))
  (bind _relativerotation (Variables|/Script/Engine.SceneComponent|GetRelativeRotation _scene))
  (bind _relativerotation_2 (Variables|/Script/Engine.SceneComponent|GetRelativeRotation _scene1))
  (bind _relativerotation_3 (Variables|/Script/Engine.SceneComponent|GetRelativeRotation _scene_2))
  (bind _relativerotation_4 (Variables|/Script/Engine.SceneComponent|GetRelativeRotation _scene1_2))
  (bind _returnvalue (Math|Interpolation|FInterpTo (.pitch _relativerotation_3) 9e+01 DeltaSeconds 5.0))
  (bind _returnvalue_2 (Math|Interpolation|FInterpTo (.pitch _relativerotation_4) -9e+01 DeltaSeconds 5.0))
  (bind _returnvalue_3 (Math|Interpolation|FInterpTo (.pitch _relativerotation) 0.0 DeltaSeconds 5.0))
  (bind _returnvalue_4 (Math|Interpolation|FInterpTo (.pitch _relativerotation_2) 0.0 DeltaSeconds 5.0))
  (if (Variables|Default|GetStartEventTick)
    (if (Variables|Default|GetIsOpening)
      (Utilities|FlowControl|Sequence
        (:then_0
          (Transformation|SetRelativeRotation _scene_2 (Math|Rotator|MakeRotator 0.0 _returnvalue 0.0) false false)
          (if (Math|Float|NearlyEqual(Float) _returnvalue 9e+01 1.0)
            (Variables|Default|SetStartEventTick false :!label _label)))
        (:then_1
          (Transformation|SetRelativeRotation _scene1_2 (Math|Rotator|MakeRotator 0.0 _returnvalue_2 0.0) false false)
          (if (Math|Float|NearlyEqual(Float) _returnvalue_2 -9e+01 -1.0)
            (goto _label))))
      (else
        (Utilities|FlowControl|Sequence
          (:then_0
            (Transformation|SetRelativeRotation _scene (Math|Rotator|MakeRotator 0.0 _returnvalue_3 0.0) false false)
            (if (Math|Float|NearlyEqual(Float) _returnvalue_3 0.0 1.0)
              (Variables|Default|SetStartEventTick false :!label _label_2)))
          (:then_1
            (Transformation|SetRelativeRotation _scene1 (Math|Rotator|MakeRotator 0.0 _returnvalue_4 0.0) false false)
            (if (Math|Float|NearlyEqual(Float) _returnvalue_4 0.0 -1.0)
              (goto _label_2))))))))

(event EventDeactivate
  (Variables|Default|SetStartEventTick true)
  (Variables|Default|SetIsOpening false))

(event EventActivate
  (Variables|Default|SetStartEventTick true)
  (Variables|Default|SetIsOpening true))

(fn ConstructionScript)