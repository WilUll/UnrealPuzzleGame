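; Player character for first-person parkour movement with sprinting, crouching, sliding, jumping, wallrunning and box carrying.
; Input drives a player-state machine that sets walk speed, resizes the capsule for crouches and zeroes ground friction during timed slides.
; While wallrunning, Tick traces sideways for "WallRun"-tagged actors, launches along the wall and rolls the camera, until jumping launches off.
; A camera trace calls IBP_Interactable, and held "Box" actors snap to GrabLocation until release.
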(event Custom|StopSlidingEvent_Event
  (Utilities|FlowControl|Delay 0.7)
  (CallFunction|StopSlide))

(event EventBeginPlay
  (Utilities|FlowControl|Sequence
    (:then_0
      (EventDispatchers|BindEventtoStopSlidingEvent (delegate Custom|StopSlidingEvent_Event)))
    (:then_1
      (Variables|Default|SetPlayerHeightHalf (Variables|/Script/Engine.CapsuleComponent|GetCapsuleHalfHeight (Variables|Collision|GetCapsuleComponent)))
      (Variables|Default|SetPlayerHeightCrouchHalf (/ (Variables|Default|GetPlayerHeightHalf) 2.0))
      (Variables|Default|SetPlayerStartGravity (Components|Movement|GetGravityZ (Variables|Character|GetCharacterMovement))))))

(event Collision|EventActorBeginOverlap
  (params (OtherActor :type Actor%20Object%20Reference)))

(event EventTick
  (params (DeltaSeconds :type Float%20%28single-precision%29))
  (bind (_left _right) (Utilities|GetLineTraceforWallRun))
  ;[0.154 1 0.86] Wallrun
  (Utilities|FlowControl|Sequence
    (:then_0
      ;[0.4173 0.2587 1] Interact
      (if (Variables|Default|GetIsInteracting)
        (Transformation|AttachComponentToComponent (Variables|Default|GetActorBeingHeld) (Variables|Default|GetGrabLocation) "None" "SnapToTarget" "SnapToTarget" "SnapToTarget" true)))
    (:then_1
      (if (Variables|Default|GetWallrunning)
        (bind (_outhit _returnvalue) (Collision|LineTraceByChannel _left _right "TraceTypeQuery1" false 0 "None"))
        (if _returnvalue
          (if (Actor|ActorHasTag (.HitActor (Collision|BreakHitResult _outhit)) "WallRun")
            (Variables|Default|SetWallNormal (.Normal (Collision|BreakHitResult _outhit)))
            (Character|LaunchCharacter (Utilities|StickPlayerOntoWall) false false)
            (Character|LaunchCharacter (* (Math|Vector|CrossProduct (Variables|Default|GetWallNormal) "0, 0,1.000000") 9e+02) true true)
            (CallFunction|WallrunTiltCamera))
          (else
            (Variables|Default|SetWallrunning false)))))
    (:then_2
      (if (not (Variables|Default|GetCorrectRotation))
        (CallFunction|WallrunUnTilt)))))

(event Input|ActionEvents|InputActionInteract
  (params (Key :type Key%20Structure :default "None"))
  (bind _camera (Variables|Default|GetCamera))
  (bind _actorbeingheld (Variables|Default|GetActorBeingHeld))
  (bind _returnvalue (Transformation|GetWorldLocation _camera))
  ;[0.4173 0.2587 1] Interact
  (:Pressed
    (bind (_outhit _returnvalue_2) (Collision|LineTraceByChannel _returnvalue (+ _returnvalue (* (Math|Vector|GetForwardVector _camera) 4e+02)) "TraceTypeQuery1" false 0 "ForDuration"))
    (if _returnvalue_2
      (if (Utilities|DoesObjectImplementInterface (.HitActor (Collision|BreakHitResult _outhit)) "/Game/Blueprint/IBP_Interactable.IBP_Interactable_C")
        (Class|IBPInteractable|Interact(Message) (.HitActor (Collision|BreakHitResult _outhit)))
        (if (Actor|ActorHasTag (.HitActor (Collision|BreakHitResult _outhit)) "Box")
          (CallFunction|GrabObject (.HitActor (Collision|BreakHitResult _outhit)))))))
  (:Released
    (if (Variables|Default|GetIsInteracting)
      (Class|IBPInteractable|Interact(Message) _actorbeingheld)
      (if (Actor|ActorHasTag _actorbeingheld "Box")
        (CallFunction|DropObject)))))

(event Input|AxisEvents|InputAxisMouseX
  (params (AxisValue :type Float%20%28single-precision%29))
  ;[1 0 0.04223] Camera
  (bind _output_get (Variables|Default|SetLookRotationX (+ AxisValue (Variables|Default|GetLookRotationX))))
  (Pawn|SetControlRotation (Game|GetPlayerController 0) (Math|Rotator|MakeRotator 0.0 0.0 _output_get)))

(event Input|AxisEvents|InputAxisMouseY
  (params (AxisValue :type Float%20%28single-precision%29))
  ;[1 0 0.04223] Camera
  (bind _output_get (Variables|Default|SetLookRotationY (Math|Float|Clamp(Float) (+ (Variables|Default|GetLookRotationY) AxisValue) -9e+01 9e+01)))
  (Transformation|SetRelativeRotation (Variables|Default|GetSpringArm) (Math|Rotator|MakeRotator 0.0 _output_get 0.0) false false))

(event Input|AxisEvents|InputAxisHorizontal
  (params (AxisValue :type Float%20%28single-precision%29))
  ;[0.8413 0.1765 1] BasicMovement
  (Class|PawnMovementComponent|AddInputVector (Variables|Character|GetCharacterMovement) (* AxisValue (Math|Vector|GetRightVector (Variables|Collision|GetCapsuleComponent))) false))

(event Input|AxisEvents|InputAxisVertical
  (params (AxisValue :type Float%20%28single-precision%29))
  ;[0.8413 0.1765 1] BasicMovement
  (Class|PawnMovementComponent|AddInputVector (Variables|Character|GetCharacterMovement) (* (Math|Vector|GetForwardVector (Variables|Collision|GetCapsuleComponent)) AxisValue) false))

(event EventOnLanded
  (params (Hit :type Hit%20Result%20Structure%20%28by%20ref%29))
  (Utilities|FlowControl|Sequence
    (:then_0
      (CallFunction|CheckNewPlayerState))
    (:then_1
      (if (Utilities|Operators|NotEqual(!=) :A (Variables|/Script/Engine.SceneComponent|GetRelativeRotation (Variables|Default|GetCamera)) :ErrorTolerance 0.01)
        (Variables|Default|SetCorrectRotation false)))))

(event Input|ActionEvents|InputActionJump
  (params (Key :type Key%20Structure))
  (:Pressed
    (Variables|Default|SetJumpKeyDown true)
    (if (AI|Components|NavMovement|IsFalling (Variables|Character|GetCharacterMovement))
      (if (Variables|Default|GetWallrunning)
        (Variables|Default|SetCorrectRotation false)
        (Utilities|LaunchfromWall)
        (else
          (CallFunction|CheckWallrun)
          (CallFunction|ChangePlayerState "NewEnumerator4")))
      (else
        (Utilities|CheckPlayerState
          (:Walking
            _)
          (:Sprinting
            _)
          (:Crouching
            _)
          (:Sliding
            _))
        (CallFunction|ChangePlayerState "NewEnumerator5"))))
  (:Released
    (Variables|Default|SetJumpKeyDown false)))

(event Input|ActionEvents|InputActionCrouch
  (params (Key :type Key%20Structure))
  (:Pressed
    (Variables|Default|SetCrouchKeyDown true)
    (Utilities|CheckPlayerState
      (:Walking
        (CallFunction|ChangePlayerState "NewEnumerator2" :!label _label))
      (:Sprinting
        (if (Variables|Default|GetCanSlide) :!label _label_2
          (CallFunction|ChangePlayerState "NewEnumerator3")
          (Variables|Default|SetCanSlide false)
          (Utilities|FlowControl|Delay 0.5)
          (Variables|Default|SetCanSlide true)
          (else
            (goto _label))))
      (:Jumping
        (goto _label_2))))
  (:Released
    (Variables|Default|SetCrouchKeyDown false)
    (CallFunction|StopCrouch)))

(event Input|ActionEvents|InputActionSprint
  (params (Key :type Key%20Structure))
  (:Pressed
    (Variables|Default|SetSprintKeyDown true)
    (Utilities|CheckPlayerState
      (:Walking
        _)
      (:Crouching
        _))
    (CallFunction|ChangePlayerState "NewEnumerator1"))
  (:Released
    (Variables|Default|SetSprintKeyDown false)
    (Utilities|CheckPlayerState
      (:Sprinting
        (CallFunction|CheckNewPlayerState)))))

(fn ConstructionScript)

(fn ChangePlayerState
  (params (ChangeTo :type ENUM_PlayerState%20Enum :default "NewEnumerator0"))
  (if (Utilities|Enum|NotEqual(Enum) ChangeTo (Variables|Default|GetPlayerStatus))
    (Variables|Default|SetOldPlayerStatus (Variables|Default|GetPlayerStatus))
    (Variables|Default|SetPlayerStatus ChangeTo)
    (CallFunction|SetPlayerStateVariables)
    (Utilities|CheckPlayerState
      (:Walking
        (Character|UnCrouch :!label _label))
      (:Sprinting
        (goto _label))
      (:Crouching
        (CallFunction|StartCrouch))
      (:Sliding
        (CallFunction|StartCrouch)
        (CallFunction|StartSlide))
      (:Wallrunning
        (CallFunction|StartWallrun))
      (:Jumping
        (Character|Jump)))))

(fn SetPlayerStateVariables
  (Utilities|FlowControl|Sequence
    (:then_0
      ;[1 0.09082 0.1605] Changes Movement Speed
      (Variables|/Script/Engine.CharacterMovementComponent|SetMaxWalkSpeed (Variables|Character|GetCharacterMovement) (Utilities|Select :Index (Variables|Default|GetPlayerStatus) :NewEnumerator0 6e+02 :NewEnumerator1 1e+03 :NewEnumerator2 3e+02 :NewEnumerator3 0.0 :NewEnumerator4 0.0 :NewEnumerator5 0.0)))))

(fn CheckNewPlayerState
  (CallFunction|ChangePlayerState (select (CallFunction|CanSprint) "NewEnumerator1" (select (CallFunction|CanStand) "NewEnumerator0" "NewEnumerator2"))))

(fn CanStand
  (if (Variables|Default|GetCrouchKeyDown)
    (return false)
    (else
      (return true))))

(fn CanSprint
  (if (Variables|Default|GetSprintKeyDown)
    (return (and (CallFunction|CanStand) (not (AI|Components|NavMovement|IsFalling (Variables|Character|GetCharacterMovement)))))
    (else
      (return false))))

(fn StartSlide
  (Variables|/Script/Engine.CharacterMovementComponent|SetGroundFriction (Variables|Character|GetCharacterMovement) 0.0)
  (Default|CallStopSlidingEvent))

(fn StartCrouch
  (Components|Capsule|SetCapsuleHalfHeight (Variables|Collision|GetCapsuleComponent) (Variables|Default|GetPlayerHeightCrouchHalf) true))

(fn StopCrouch
  (Components|Capsule|SetCapsuleHalfHeight (Variables|Collision|GetCapsuleComponent) (Variables|Default|GetPlayerHeightHalf) true)
  (CallFunction|CheckNewPlayerState))

(fn StopSlide
  (Variables|/Script/Engine.CharacterMovementComponent|SetGroundFriction (Variables|Character|GetCharacterMovement) 8.0)
  (CallFunction|CheckNewPlayerState))

(fn CheckforSlide
  (return (and (Variables|Default|GetSprintKeyDown) (Variables|Default|GetCrouchKeyDown))))

(fn CheckWallrun
  (bind (_left _right) (Utilities|GetLineTraceforWallRun))
  (bind (_outhit _returnvalue) (Collision|LineTraceByChannel _left _right "TraceTypeQuery1" false 0 "None"))
  (if _returnvalue
    (if (Actor|ActorHasTag (.HitActor (Collision|BreakHitResult _outhit)) "WallRun")
      (Variables|Default|SetWallNormal (.Normal (Collision|BreakHitResult _outhit)))
      (return true)
      (else
        _)))
  (return false))

(fn StopWallrun)

(fn StartWallrun
  (Variables|Default|SetWallrunning true))

(fn WallrunTiltCamera
  (bind _camera (Variables|Default|GetCamera))
  (bind _camera_2 (Variables|Default|GetCamera))
  (bind _relativerotation (Variables|/Script/Engine.SceneComponent|GetRelativeRotation _camera))
  (bind _relativerotation_2 (Variables|/Script/Engine.SceneComponent|GetRelativeRotation _camera_2))
  (bind (_roll _pitch _yaw) (Math|Rotator|BreakRotator _relativerotation_2))
  (bind (_roll_2 _pitch_2 _yaw_2) (Math|Rotator|BreakRotator _relativerotation))
  (bind (_outhit _returnvalue) (Collision|LineTraceByChannel (Transformation|GetWorldLocation (Variables|Collision|GetCapsuleComponent)) (.Left (Utilities|GetLineTraceforWallRun)) "TraceTypeQuery1" false 0 "None"))
  (if _returnvalue
    (if (Actor|ActorHasTag (.HitActor (Collision|BreakHitResult _outhit)) "WallRun")
      (Transformation|SetRelativeRotation (Variables|Default|GetCamera) (Math|Interpolation|RInterpTo _relativerotation_2 (Math|Rotator|MakeRotator -15.0 _pitch _yaw) (Utilities|Time|GetWorldDeltaSeconds) 1e+01) false false))
    (else
      (Transformation|SetRelativeRotation (Variables|Default|GetCamera) (Math|Interpolation|RInterpTo _relativerotation (Math|Rotator|MakeRotator 15.0 _pitch_2 _yaw_2) (Utilities|Time|GetWorldDeltaSeconds) 1e+01) false false))))

(fn WallrunUnTilt
  (bind _camera (Variables|Default|GetCamera))
  (bind _relativerotation (Variables|/Script/Engine.SceneComponent|GetRelativeRotation _camera))
  (bind (_roll _pitch _yaw) (Math|Rotator|BreakRotator _relativerotation))
  (Transformation|SetRelativeRotation (Variables|Default|GetCamera) (Math|Interpolation|RInterpTo _relativerotation (Math|Rotator|MakeRotator 0.0 _pitch _yaw) (Utilities|Time|GetWorldDeltaSeconds) 1e+01) false false)
  (if (Utilities|Operators|EqualEqual :A (Variables|/Script/Engine.SceneComponent|GetRelativeRotation (Variables|Default|GetCamera)) :ErrorTolerance 0.01)
    (Variables|Default|SetCorrectRotation true)))

(fn GrabObject
  (params (ObjectToGrab :type Actor%20Object%20Reference))
  (Variables|Default|SetIsInteracting true)
  (Variables|Default|SetActorBeingHeld ObjectToGrab))

(fn DropObject
  (Transformation|DetachFromActor (Variables|Default|GetActorBeingHeld) "KeepWorld" "KeepWorld" "KeepWorld")
  (Variables|Default|SetIsInteracting false)
  (Variables|Default|SetActorBeingHeld 0))

(fn Interact
  (return false))