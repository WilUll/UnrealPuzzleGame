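; Main menu camera actor that slowly pans its Camera back and forth across a quarter turn, judging by its name as a menu backdrop.
; Each Tick eases the camera's relative yaw with FInterpTo toward either zero or ninety degrees, with pitch and roll held at zero.
; The RotateBack flag picks the target and flips when the yaw nears it, producing an endless sweep that slows at each end.
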(event EventBeginPlay)

(event Collision|EventActorBeginOverlap
  (params (OtherActor :type Actor%20Object%20Reference)))

(event EventTick
  (params (DeltaSeconds :type Float%20%28single-precision%29))
  (bind _returnvalue (Utilities|Time|GetWorldDeltaSeconds))
  (bind _returnvalue_2 (Utilities|Time|GetWorldDeltaSeconds))
  (bind _camera (Variables|Default|GetCamera))
  (bind _camera_2 (Variables|Default|GetCamera))
  (bind _relativerotation (Variables|/Script/Engine.SceneComponent|GetRelativeRotation _camera))
  (bind _relativerotation_2 (Variables|/Script/Engine.SceneComponent|GetRelativeRotation _camera_2))
  (bind _returnvalue_3 (Math|Interpolation|FInterpTo (.yaw _relativerotation) 0.0 _returnvalue_2 0.5))
  (bind _returnvalue_4 (Math|Interpolation|FInterpTo (.yaw _relativerotation_2) 9e+01 _returnvalue 0.5))
  (if (Variables|Default|GetRotateBack)
    (Transformation|SetRelativeRotation _camera (Math|Rotator|MakeRotator 0.0 0.0 _returnvalue_3) false false)
    (if (Math|Float|NearlyEqual(Float) _returnvalue_3 0.0 0.5)
      (Variables|Default|SetRotateBack false))
    (else
      (Transformation|SetRelativeRotation _camera_2 (Math|Rotator|MakeRotator 0.0 0.0 _returnvalue_4) false false)
      (if (Math|Float|NearlyEqual(Float) _returnvalue_4 9e+01 0.5)
        (Variables|Default|SetRotateBack true)))))

(fn ConstructionScript)